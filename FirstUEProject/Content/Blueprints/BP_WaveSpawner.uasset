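; BP_WaveSpawner is an enemy wave spawner that starts a wave on BeginPlay.
; SpawnWave increments CurrentWave, reads that wave's enemy count from the values of Waves, and spawns that many BP_Enemy at its own transform.
; Tick gathers all BP_Enemy every frame, but its branch is fixed false and the empty-list check is unconnected, so later waves never start.
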(event Custom|Spawn%20Wave
  (Math|Integer|IncrementInt (Variables|Default|GetCurrent%20Wave)
    (:%20%20
      (bind _values (Utilities|Map|Values (Variables|Default|GetWaves)))
      (for _index (range 1 (Utilities|Array|Get(acopy) _values (- (Variables|Default|GetCurrent%20Wave) 1)))
        (Game|SpawnActorfromClass "/Game/Blueprints/BP_Enemy.BP_Enemy_C" (Transformation|GetActorTransform) "AdjustIfPossibleButAlwaysSpawn" "MultiplyWithRoot" 0 0)))))

(event EventBeginPlay
  (CallFunction|SpawnWave))

(event EventTick
  (params (DeltaSeconds :type Float%20%28single-precision%29))
  (bind _outactors (Actor|GetAllActorsOfClass "/Game/Blueprints/BP_Enemy.BP_Enemy_C"))
  (if false
    (CallFunction|SpawnWave)))

(fn ConstructionScript)